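; PendiumBP is an actor that swings its Spinner component back and forth in yaw, like a pendulum.
; Each Tick adds delta time scaled by Mag to Accumulator, then sets Spinner's relative yaw to that value's cosine times Speed.
; Mag therefore sets the swing rate and Speed the amplitude in degrees.
; A graph comment notes that replication periodically corrects drift between server and clients caused by differing delta times.
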(event EventBeginPlay)

(event Collision|EventActorBeginOverlap
  (params (OtherActor :type Actor%20Object%20Reference)))

(event EventTick
  (params (DeltaSeconds :type Float%20%28single-precision%29))
  (bind _output_get (Variables|Default|SetAccumulator (+ (* DeltaSeconds (Variables|Default|GetMag)) (Variables|Default|GetAccumulator)))) ; Replicated so server will send updates every so often to keep clients/server in sync (given delta time won't be in sync)
  (Transformation|SetRelativeRotation (Variables|Default|GetSpinner) (Math|Rotator|MakeRotator 0.0 0.0 (* (Math|Trig|Cos(Degrees) _output_get) (Variables|Default|GetSpeed))) false false))

(fn ConstructionScript)