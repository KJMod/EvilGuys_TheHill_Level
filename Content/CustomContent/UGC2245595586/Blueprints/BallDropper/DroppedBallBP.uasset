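; DroppedBallBP is a dropped ball actor that knocks characters it hits and despawns on the server after a fixed lifetime.
; On spawn it picks a random colour material for the second mesh slot, and clients start its audio after a short delay.
; A mesh hit launches any Character at the ball's velocity, overriding its own.
; Every tick, speed drives audio volume and pitch through float curves.
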(event OnComponentHit(StaticMesh)
  (params (HitComponent :type Primitive%20Component%20Object%20Reference) (OtherActor :type Actor%20Object%20Reference) (OtherComp :type Primitive%20Component%20Object%20Reference) (NormalImpulse :type Vector :default "0, 0, 0") (Hit :type Hit%20Result%20Structure%20%28by%20ref%29))
  ;[1 1 1] Simple knock on impact
  (bind _ascharacter (Utilities|Casting|CastToCharacter OtherActor))
  (Character|LaunchCharacter _ascharacter (* (Transformation|GetVelocity) 1.0) true true))

(event EventBeginPlay
  (Audio|Components|Audio|Stop (Variables|Default|GetAudio))
  (Rendering|Material|SetMaterial (Variables|Default|GetStaticMesh) 1 (Utilities|Select :Index (Math|Random|RandomIntegerinRange 0 5) :Option%200 "/Game/CustomContent/UGC2245595586/Materials/M_Blue.M_Blue" :Option%201 "/Game/CustomContent/UGC2245595586/Materials/M_Red.M_Red" :Option%202 "/Game/CustomContent/UGC2245595586/Materials/M_Orange.M_Orange" :Option%203 "/Game/CustomContent/UGC2245595586/Materials/M_Yellow.M_Yellow" :Option%204 "/Game/CustomContent/UGC2245595586/Materials/M_Purple.M_Purple" :Option%205 "/Game/CustomContent/UGC2245595586/Materials/M_Green.M_Green"))
  (Networking|SwitchHasAuthority
    (:Authority
      (Utilities|FlowControl|Delay 25.0)
      (Actor|DestroyActor))
    (:Remote
      (Utilities|FlowControl|Delay 1.5)
      (Audio|Components|Audio|Play (Variables|Default|GetAudio) 0.0))))

(event EventTick
  (params (DeltaSeconds :type Float%20%28single-precision%29))
  (bind _returnvalue (Transformation|GetVelocity))
  (bind _audio (Variables|Default|GetAudio))
  (bind _returnvalue_2 (Math|Vector|VectorLength _returnvalue))
  (Audio|Components|Audio|SetVolumeMultiplier _audio (Math|Curves|GetFloatValue (Variables|Default|GetVolCurveFloat) _returnvalue_2) :!class /Script/Engine.AudioComponent)
  (Audio|Components|Audio|SetPitchMultiplier _audio (Math|Curves|GetFloatValue (Variables|Default|GetPitchCurveFloat) _returnvalue_2)))

(fn ConstructionScript)