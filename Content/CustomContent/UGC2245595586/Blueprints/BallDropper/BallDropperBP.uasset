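; BallDropperBP is a dropper actor that repeatedly spawns DroppedBallBP balls at its own transform, always spawning regardless of collision.
; BeginPlay sets a short random initial delay to stagger the first drop.
; On authority only, Tick feeds a latent Delay that serves as the repeat timer.
; Each time it completes, it rerolls the delay between MinDelay and MaxDelay and spawns a ball.
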(event EventBeginPlay
  (Variables|Default|SetRandomDelay (Math|Random|RandomFloatinRange 0.0 5.0)))

(event EventTick
  (params (DeltaSeconds :type Float%20%28single-precision%29))
  (Networking|SwitchHasAuthority
    (:Authority
      (Utilities|FlowControl|Delay (Variables|Default|GetRandomDelay))
      (Variables|Default|SetRandomDelay (Math|Random|RandomFloatinRange (Variables|Default|GetMinDelay) (Variables|Default|GetMaxDelay)))
      (Game|SpawnActorfromClass "/Game/CustomContent/UGC2245595586/Blueprints/BallDropper/DroppedBallBP.DroppedBallBP_C" (Transformation|GetActorTransform) "AlwaysSpawn" 0 0))))

(fn ConstructionScript)