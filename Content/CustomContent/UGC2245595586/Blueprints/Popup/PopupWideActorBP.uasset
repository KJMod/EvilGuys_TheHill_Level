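; PopupWideActorBP is an actor with a Popup component that repeatedly moves vertically at random intervals.
; BeginPlay gives it a random material from six striped variants or six solid colors, depending on DarkScheme, and sets a short random initial delay.
; On authority, Tick runs a Delay as a loop, rerolling the interval between MinDelay and MaxDelay and calling FireEvent.
; FireEvent plays PopupTimeline, which drives the component's relative Z with teleporting, unswept moves.
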(event Custom|FireEvent
  (bind _newtrack_0 (Timeline|PopupTimeline PlayFromStart)
    (:Update
      (Transformation|SetRelativeLocation (Variables|Default|GetPopup) (Math|Vector|MakeVector 0.0 0.0 _newtrack_0) false true))))

(event EventBeginPlay
  (bind _returnvalue (Math|Random|RandomIntegerinRange 0 5))
  (Rendering|Material|SetMaterial (Variables|Default|GetPopup) 0 (select (Variables|Default|GetDarkScheme) (Utilities|Select :Index _returnvalue :Option%200 "/Game/CustomContent/UGC2245595586/Materials/Dark/Stripes/Dark_Stripes_Mat_Inst.Dark_Stripes_Mat_Inst" :Option%201 "/Game/CustomContent/UGC2245595586/Materials/Dark/Stripes/Dark_Stripes_Mat_Inst1.Dark_Stripes_Mat_Inst1" :Option%202 "/Game/CustomContent/UGC2245595586/Materials/Dark/Stripes/Dark_Stripes_Mat_Inst2.Dark_Stripes_Mat_Inst2" :Option%203 "/Game/CustomContent/UGC2245595586/Materials/Dark/Stripes/Dark_Stripes_Mat_Inst3.Dark_Stripes_Mat_Inst3" :Option%204 "/Game/CustomContent/UGC2245595586/Materials/Dark/Stripes/Dark_Stripes_Mat_Inst4.Dark_Stripes_Mat_Inst4" :Option%205 "/Game/CustomContent/UGC2245595586/Materials/Dark/Stripes/Dark_Stripes_Mat_Inst5.Dark_Stripes_Mat_Inst5") (Utilities|Select :Index _returnvalue :Option%200 "/Game/CustomContent/UGC2245595586/Materials/M_Blue.M_Blue" :Option%201 "/Game/CustomContent/UGC2245595586/Materials/M_Red.M_Red" :Option%202 "/Game/CustomContent/UGC2245595586/Materials/M_Orange.M_Orange" :Option%203 "/Game/CustomContent/UGC2245595586/Materials/M_Yellow.M_Yellow" :Option%204 "/Game/CustomContent/UGC2245595586/Materials/M_Purple.M_Purple" :Option%205 "/Game/CustomContent/UGC2245595586/Materials/M_Green.M_Green")))
  (Variables|Default|SetRandomDelay (Math|Random|RandomFloatinRange 0.0 1.0)))

(event EventTick
  (params (DeltaSeconds :type Float%20%28single-precision%29))
  (Networking|SwitchHasAuthority
    (:Authority
      (Utilities|FlowControl|Delay (Variables|Default|GetRandomDelay))
      (Variables|Default|SetRandomDelay (Math|Random|RandomFloatinRange (Variables|Default|GetMinDelay) (Variables|Default|GetMaxDelay)))
      (CallFunction|FireEvent))))

(fn ConstructionScript)